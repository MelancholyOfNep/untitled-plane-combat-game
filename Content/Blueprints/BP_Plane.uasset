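; Player-flown plane with throttle, flight controls, cannon, missiles and target lock, plus mission HUD, pause menu and failure screen.
; Tick pushes the physics body forward and bends its velocity toward the nose, tipping it down below stall speed; maneuverability peaks near 80% throttle.
; Cannon fires on a looping timer, missiles have a cooldown, and lock-on sphere-traces for enemies.
; Any hit deals self-damage; zero health triggers explosion and mission failure.
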(event Input|EnhancedActionEvents|EnhancedInputActionIA_Throttle
  (params (ActionValue :type Float%20%28double-precision%29) (ElapsedSeconds :type Float%20%28double-precision%29) (TriggeredSeconds :type Float%20%28double-precision%29) (InputAction :type Input%20Action%20Object%20Reference :default "/Game/Input/IA_Throttle.IA_Throttle"))
  (bind _maxforwardvelocity (Variables|Default|GetMaxForwardVelocity))
  ;[1 1 1] Throttle Control
  (bind _output_get (Variables|Default|SetCurrentForwardVelocity (Math|Float|Clamp(Float) (+ (* ActionValue 1e+02 (Utilities|Time|GetWorldDeltaSeconds)) (Variables|Default|GetCurrentForwardVelocity)) 0.0 _maxforwardvelocity)))
  (bind _output_get_2 (Variables|Default|SetManeuverability (* (- 1.0 (Math|Float|Absolute(Float) (- 1.0 (/ _output_get (* _maxforwardvelocity 0.8))))) (Variables|Default|GetDefaultManeuverability)))))

(event Input|EnhancedActionEvents|EnhancedInputActionIA_Move
  (params (ActionValue :type Vector :default "0, 0, 0") (ElapsedSeconds :type Float%20%28double-precision%29) (TriggeredSeconds :type Float%20%28double-precision%29) (InputAction :type Input%20Action%20Object%20Reference :default "/Game/Input/IA_Move.IA_Move"))
  ;[1 1 1] Pitch, Roll, Yaw
  (:Triggered
    (Transformation|AddActorLocalRotation (Math|Rotator|MakeRotator (* (.x ActionValue) 2.0) (* (.y ActionValue) (Variables|Default|GetManeuverability)) (* (.z ActionValue) 0.15)) false false)
    (Variables|Default|SetAnimRoll (.x ActionValue) :!label _label)
    (Variables|Default|SetAnimPitch (.y ActionValue)))
  (:Completed
    (goto _label)))

(event Input|EnhancedActionEvents|EnhancedInputActionIA_Airbrake
  (params (ActionValue :type Boolean) (ElapsedSeconds :type Float%20%28double-precision%29) (TriggeredSeconds :type Float%20%28double-precision%29) (InputAction :type Input%20Action%20Object%20Reference :default "/Game/Input/IA_Airbrake.IA_Airbrake"))
  ;[1 1 1] Airbraking. Needs to be either reworked or removed.
)

(event Input|EnhancedActionEvents|EnhancedInputActionIA_Pause
  (params (ActionValue :type Boolean) (ElapsedSeconds :type Float%20%28double-precision%29) (TriggeredSeconds :type Float%20%28double-precision%29) (InputAction :type Input%20Action%20Object%20Reference :default "/Game/Input/IA_Pause.IA_Pause"))
  (bind _returnvalue (Game|GetPlayerController 0))
  ;[1 1 1] Pause & quit
  (:Started
    (if (Game|IsGamePaused)
      (Game|SetGamePaused false)
      (Input|SetInputModeGameOnly _returnvalue true)
      (Widget|RemovefromParent (stale _returnvalue_2))
      (Variables|/Script/Engine.PlayerController|SetbShowMouseCursor _returnvalue false)
      (else
        (Game|SetGamePaused true)
        (bind _returnvalue_2 (UserInterface|CreateWidget "/Game/Blueprints/Menus/WBP_Pause.WBP_Pause_C"))
        (Input|SetInputModeUIOnly _returnvalue _returnvalue_2 "LockInFullscreen" true)
        (UserInterface|Viewport|AddtoViewport _returnvalue_2 0)
        (Variables|/Script/Engine.PlayerController|SetbShowMouseCursor _returnvalue true)))))

(event Input|EnhancedActionEvents|EnhancedInputActionIA_Cannon
  (params (ActionValue :type Boolean) (ElapsedSeconds :type Float%20%28double-precision%29) (TriggeredSeconds :type Float%20%28double-precision%29) (InputAction :type Input%20Action%20Object%20Reference :default "/Game/Input/IA_Cannon.IA_Cannon"))
  (:Started
    (bind _returnvalue (Audio|SpawnSoundAttached "/Game/Audio/SFX/611449__seidhepriest__m61a2-minigun.611449__seidhepriest__m61a2-minigun" (Variables|Default|GetCube) "None" "0, 0, 0" "0, 0, 0" "KeepRelativeOffset" true 1.0 1.0 0.0 0 0))
    (CallFunction|CannonFire)
    (bind _returnvalue_2 (Utilities|Time|SetTimerbyFunctionName 0 "CannonFire" 0.04 true)))
  (:Completed
    (Utilities|Time|ClearandInvalidateTimerbyHandle _returnvalue_2)
    (Audio|Components|Audio|Stop _returnvalue)))

(event Input|EnhancedActionEvents|EnhancedInputActionIA_LockOn
  (params (ActionValue :type Boolean) (ElapsedSeconds :type Float%20%28double-precision%29) (TriggeredSeconds :type Float%20%28double-precision%29) (InputAction :type Input%20Action%20Object%20Reference :default "/Game/Input/IA_LockOn.IA_LockOn"))
  (bind _cube (Variables|Default|GetCube))
  (bind _returnvalue (Transformation|GetWorldLocation _cube))
  (bind _returnvalue_2 (Math|Vector|GetForwardVector _cube))
  (bind _outactors (Actor|GetAllActorsOfClass "/Script/Landscape.LandscapeProxy"))
  (bind _outhit (Collision|SphereTraceForObjects (+ (* _returnvalue_2 1e+01) _returnvalue) (+ _returnvalue (* _returnvalue_2 1e+05)) 7.5e+02 (Variables|Default|GetObject%20Types) false _outactors "ForOneFrame"))
  (if (Utilities|ClassIsChildOf (Utilities|GetClass (.hitactor _outhit)) "/Game/Blueprints/Targets/BP_EnemyTest.BP_EnemyTest_C")
    (CallFunction|LockTarget (.hitactor _outhit) :!label _label)
    (bind _asbp_enemy_test (Utilities|Casting|CastToBP_EnemyTest (.hitactor _outhit))
      (:then
        (Default|Locked _asbp_enemy_test))
      (:CastFailed
        (bind _asbp_patrol_enemy (Utilities|Casting|CastToBP_Patrol_enemy (.hitactor _outhit)))
        (Default|Locked _asbp_patrol_enemy)))
    (Development|PrintString (Utilities|String|Append "Locked: " (Utilities|GetDisplayName (.hitactor _outhit))))
    (elif (Utilities|ClassIsChildOf (Utilities|GetClass (.hitactor _outhit)) "/Game/Blueprints/Targets/BP_Patrol_enemy.BP_Patrol_enemy_C")
      (goto _label)
      (else
        (Development|PrintString "No target found.")))))

(event Input|EnhancedActionEvents|EnhancedInputActionIA_Missile
  (params (ActionValue :type Boolean) (ElapsedSeconds :type Float%20%28double-precision%29) (TriggeredSeconds :type Float%20%28double-precision%29) (InputAction :type Input%20Action%20Object%20Reference :default "/Game/Input/IA_Missile.IA_Missile"))
  (:Started
    (if (not (Variables|Default|GetMissileCooldown?))
      (if (>= (Variables|Default|GetSpecialAmmo1) 1)
        (Audio|SpawnSoundAttached "/Game/Audio/SFX/MissileLaunch.MissileLaunch" (Variables|Default|GetCube) "None" "0, 0, 0" "0, 0, 0" "KeepRelativeOffset" false 0.5 1.0 0.0 0 0)
        (bind _returnvalue (Game|SpawnActorfromClass "/Game/Blueprints/BP_Missile.BP_Missile_C" (Transformation|GetWorldTransform (Variables|Default|GetArrow)) "Undefined" "MultiplyWithRoot" 0 0))
        (Audio|SpawnSoundAttached "/Game/Audio/SFX/EngineSound.EngineSound" (Class|Actor|GetParentComponent _returnvalue) "None" "0, 0, 0" "0, 0, 0" "KeepRelativeOffset" false 1.0 1.0 0.0 0 0)
        (bind _result (Math|Integer|DecrementInt (Variables|Default|GetSpecialAmmo1))
          (:%20%20
            (Variables|/Game/Blueprints/HUD/WBP_HUDMission.WBP_HUDMission_C|SetMissileCountText (Variables|Default|GetBP_HUDMission) (Utilities|Text|ToText(Integer) _result))
            (Variables|Default|SetMissileCooldown? true)
            (Utilities|FlowControl|Delay 1.0)
            (Variables|Default|SetMissileCooldown? false)))))))

(event EventBeginPlay
  (|CallParentFunction)
  (bind _asbp_game_instance (Utilities|Casting|CastToBP_GameInstance (Game|GetGameInstance)))
  (Input|SetInputModeGameOnly (Game|GetPlayerController 0) false)
  (Default|Load _asbp_game_instance)
  (CameraFades|StartCameraFade :self (Game|GetPlayerCameraManager 0) :FromAlpha 1.0 :Duration 5.0 :bShouldFadeAudio true)
  (bind _returnvalue (UserInterface|CreateWidget "/Game/Blueprints/HUD/WBP_HUDMission.WBP_HUDMission_C"))
  (UserInterface|Viewport|AddtoViewport _returnvalue 0)
  (bind _output_get (Variables|Default|SetBP_HUDMission _returnvalue))
  (Variables|/Game/Blueprints/HUD/WBP_HUDMission.WBP_HUDMission_C|SetAmmoCountText _output_get (Utilities|Text|ToText(Integer) (Variables|Default|GetCannonAmmo)))
  (Variables|/Game/Blueprints/HUD/WBP_HUDMission.WBP_HUDMission_C|SetHealthCountText _output_get (Utilities|Text|ToText(String) (Class|KismetMathLibrary|Round64 (Variables|Default|GetHealth))))
  (Variables|/Game/Blueprints/HUD/WBP_HUDMission.WBP_HUDMission_C|SetMissileCountText _output_get (Utilities|Text|ToText(Integer) (Variables|Default|GetSpecialAmmo1)))
  (bind _returnvalue_2 (Audio|SpawnSoundAttached "/Game/Audio/SFX/EngineSound.EngineSound" (Variables|Default|GetCube) "None" "0, 0, 0" "0, 0, 0" "KeepRelativeOffset" true 0.35 1.0 0.0 0 0))
  (Variables|Default|SetJetNoise _returnvalue_2)
  ;[1 1 1] Add player bindings for enhanced input
  (bind _asplayer_controller (Utilities|Casting|CastToPlayerController (Pawn|GetController)))
  (Utilities|IsValid (PlayerController|LocalPlayerSubsystems|GetEnhancedInputLocalPlayerSubsystem _asplayer_controller)
    (:Is%20Valid
      (Input|AddMappingContext (PlayerController|LocalPlayerSubsystems|GetEnhancedInputLocalPlayerSubsystem _asplayer_controller) "/Game/Input/PlaneMapping.PlaneMapping" 0 "(bIgnoreAllPressedKeysUntilRelease=True,bForceImmediately=False,bNotifyUserSettings=False)")
      (Variables|Default|SetManeuverability (* (- 1.0 (Math|Float|Absolute(Float) (- 1.0 (/ (stale Input|EnhancedActionEvents|EnhancedInputActionIA_Throttle _output_get) (* (Variables|Default|GetMaxForwardVelocity) 0.8))))) (Variables|Default|GetDefaultManeuverability))))
    (:Is%20Not%20Valid
      (Development|PrintString "Fucking player bindings died"))))

(event Collision|EventActorBeginOverlap
  (params (OtherActor :type Actor%20Object%20Reference))
  (|CallParentFunction OtherActor) ; This node is disabled and will not be called.\nDrag off pins to build functionality.
)

(event EventTick
  (params (DeltaSeconds :type Float%20%28single-precision%29))
  (bind _returnvalue (Transformation|GetActorRotation))
  ;[1 1 1] Apply forward "thrust" (just offsetting the model)
  (|CallParentFunction DeltaSeconds)
  (Physics|AddForce (Variables|Default|GetCube) (* (* (Transformation|GetActorForwardVector) (Variables|Default|GetCurrentForwardVelocity)) 1e+04) "None" false)
  (if (>= (Variables|Default|GetCurrentForwardVelocity) 5e+01)
    (Physics|SetPhysicsLinearVelocity (Variables|Default|GetCube) (Class|KismetMathLibrary|VectorSlerpVectortoDirection (Transformation|GetVelocity) (Transformation|GetActorForwardVector) 0.999) false "None")
    (else
      ;;[1 1 1] Stall
      (Transformation|SetActorRelativeRotation (Math|Rotator|Lerp(Rotator) (Math|Rotator|MakeRotator (.roll _returnvalue) (.pitch _returnvalue) (.yaw _returnvalue)) (Math|Rotator|MakeRotator 0.0 -9e+01 (.yaw _returnvalue)) 0.01 true)))))

(event Collision|EventHit
  (params (MyComp :type Primitive%20Component%20Object%20Reference) (Other :type Actor%20Object%20Reference) (OtherComp :type Primitive%20Component%20Object%20Reference) (bSelfMoved :type Boolean) (HitLocation :type Vector :default "0, 0, 0") (HitNormal :type Vector :default "0, 0, 0") (NormalImpulse :type Vector :default "0, 0, 0") (Hit :type Hit%20Result%20Structure%20%28by%20ref%29))
  (Development|PrintString "Boom")
  (Game|Damage|ApplyDamage self 1e+02 0 0))

(event Game|Damage|EventAnyDamage
  (params (Damage :type Float%20%28single-precision%29) (DamageType :type Damage%20Type%20Object%20Reference) (InstigatedBy :type Controller%20Object%20Reference) (DamageCauser :type Actor%20Object%20Reference))
  (bind _returnvalue (Game|GetPlayerController 0))
  (bind _output_get (Variables|Default|SetHealth (- (stale _output_get) Damage)))
  (Audio|PlaySound2D "/Game/Audio/SFX/702245__inmotionaudio__gunartl_69thfieldartillerygun01_inmotionaudio_freesamplesunday.702245__inmotionaudio__gunartl_69thfieldartillerygun01_inmotionaudio_freesamplesunday" 1.0 1.0 0.0 0 0)
  (Variables|/Game/Blueprints/HUD/WBP_HUDMission.WBP_HUDMission_C|SetHealthCountText (Variables|Default|GetBP_HUDMission) (Utilities|Text|ToText(String) (Utilities|String|Append "HULL: " (Utilities|String|ToString(Integer) (Class|KismetMathLibrary|Round64 _output_get)))))
  (if (<= _output_get 0.0)
    (Collision|SetCollisionEnabled (Variables|Default|GetCube) "NoCollision")
    (Pawn|UnPossess (Pawn|GetController))
    (Effects|SpawnEmitteratLocation "/Game/StarterContent/Particles/P_Explosion.P_Explosion" (Transformation|GetWorldLocation (Variables|Default|GetCube)) "0, 0, 0" "100.000000,100.000000,100.000000")
    (Utilities|FlowControl|Delay 2.0)
    (bind _returnvalue_2 (UserInterface|CreateWidget "/Game/Blueprints/Menus/WBP_MissionFailed.WBP_MissionFailed_C"))
    (UserInterface|Viewport|AddtoViewport _returnvalue_2 0)
    (Variables|/Script/Engine.PlayerController|SetbShowMouseCursor _returnvalue true)
    (Input|SetInputModeUIOnly _returnvalue _returnvalue_2 "DoNotLock" false)
    (Utilities|Time|SetGlobalTimeDilation 0.0)
    (else
      (bind _returnvalue_3 (UserInterface|CreateWidget "/Game/Blueprints/HUD/WBP_Hurt.WBP_Hurt_C"))
      (UserInterface|Viewport|AddtoViewport _returnvalue_3 0)
      (Utilities|FlowControl|Delay 0.1)
      (Widget|RemovefromParent _returnvalue_3))))

(event Input|KeyboardEvents|DebugKeyF5
  (params (Key :type Key%20Structure :default "None") (ActionValue :type Input%20Action%20Value%20Structure))
  (:Pressed
    (bind _asbp_game_instance (Utilities|Casting|CastToBP_GameInstance (Game|GetGameInstance)))
    (Default|Save _asbp_game_instance)))

(event Input|KeyboardEvents|DebugKeyTab
  (params (Key :type Key%20Structure :default "None") (ActionValue :type Input%20Action%20Value%20Structure))
  (:Pressed
    (Game|OpenLevel(byName) "Testbed")))

(fn ConstructionScript)

(fn CannonFire
  (bind _cube (Variables|Default|GetCube))
  (if (>= (Variables|Default|GetCannonAmmo) 1)
    (Game|SpawnActorfromClass "/Game/Blueprints/BP_Bullet.BP_Bullet_C" (Math|Transform|MakeTransform (+ (+ (* (Math|Vector|GetForwardVector (Variables|Default|GetCube)) 1e+02) (* (Math|Vector|GetUpVector (Variables|Default|GetCube)) -1e+02)) (Transformation|GetSocketLocation _cube "None")) (Transformation|GetWorldRotation _cube)) "Undefined" "MultiplyWithRoot" 0 (+ (Math|Vector|VectorLength (Transformation|GetVelocity)) 2e+04) self)
    (Effects|SpawnEmitteratLocation "/Game/StarterContent/Particles/P_Explosion.P_Explosion" (Transformation|GetWorldLocation (Variables|Default|GetGunExplLoc)) "0, 0, 0" "0.500000,0.500000,0.500000" false)
    (bind _result (Math|Integer|DecrementInt (Variables|Default|GetCannonAmmo))
      (:%20%20
        (Variables|/Game/Blueprints/HUD/WBP_HUDMission.WBP_HUDMission_C|SetAmmoCountText (Variables|Default|GetBP_HUDMission) (Utilities|Text|ToText(Integer) _result))))))

(fn LockTarget
  (params (NewLockedActor :type Actor%20Object%20Reference))
  (bind _asbp_enemy_test (Utilities|Casting|CastToBP_EnemyTest (Variables|Default|GetLockedTarget))
    (:then
      (Default|Unlocked _asbp_enemy_test))
    (:CastFailed
      (bind _asbp_patrol_enemy (Utilities|Casting|CastToBP_Patrol_enemy (Variables|Default|GetLockedTarget))
        (:then
          (Default|Unlocked _asbp_patrol_enemy))
        (:CastFailed
          _))))
  (Variables|Default|SetLockedTarget NewLockedActor))