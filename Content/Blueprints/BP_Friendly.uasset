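; BP_Friendly is a destructible friendly actor that costs the player money when destroyed.
; On BeginPlay it tints its HUD marker widget a translucent blue.
; AnyDamage lowers Health; at zero or below it destroys the actor, subtracts its Value from Money in BP_GameInstance, prints the new total and plays an explosion sound.
; It then clears the player BP_Plane's LockedTarget if that lock points at itself.
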(event `self.ReceiveBeginPlay`
  (`KismetSystemLibrary.PrintString` "Hello")
  (`UserWidget.SetColorAndOpacity` (`WidgetComponent.GetUserWidgetObject` (`self.HUDmarker`)) (struct :`G` 0.546725 :`B` 1.0 :`A` 0.75)))

(event `self.ReceiveAnyDamage`
  (params (Damage :type "Float (single-precision)") (DamageType :type "DamageType Object Reference") (InstigatedBy :type "Controller Object Reference") (DamageCauser :type "Actor Object Reference"))
  (bind _output_get (set `self.Health` (- (stale _output_get) Damage)))
  (if (<= _output_get 0.0)
    (`self.K2_DestroyActor`)
    (bind _asbp_game_instance (cast `/Game/Blueprints/BP_GameInstance` (`GameplayStatics.GetGameInstance`)))
    (bind _output_get_2 (set `/Game/Blueprints/BP_GameInstance.Money` (- (stale _output_get_2) (`self.Value`)) _asbp_game_instance))
    (`KismetSystemLibrary.PrintString` (`KismetStringLibrary.Concat_StrStr` "Friendly Destroyed! Money: " (`KismetStringLibrary.Conv_IntToString` _output_get_2)))
    (`GameplayStatics.PlaySoundAtLocation` "/Game/StarterContent/Audio/Explosion01.Explosion01" (`SceneComponent.K2_GetComponentLocation` (`self.Box`)) (struct) 1.0 1.0 0.0 null null null null)
    (bind _asbp_plane (cast `/Game/Blueprints/BP_Plane` (`GameplayStatics.GetPlayerPawn` 0)))
    (if (== (`/Game/Blueprints/BP_Plane.LockedTarget` _asbp_plane) self)
      (set `/Game/Blueprints/BP_Plane.LockedTarget` null _asbp_plane))))

(fn `UserConstructionScript`)