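; Test enemy child Blueprint that acts as an anti-air shooter against BP_Plane.
; A plane entering the PlayerNearby volume starts a looping AAFire timer, and leaving clears it.
; AAFire predicts a launch vector toward player pawn 0 with SuggestProjectileVelocityMovingTarget, using only its direction to spawn fixed-speed BP_Enemy_Bullet actors at the Arrow, plus smoke.
; The prediction leaves persistent debug drawing on, and the stored Player reference goes unused in aiming.
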(event `self.PlayerNearby.OnComponentBeginOverlap`
  (params (OverlappedComponent :type "PrimitiveComponent Object Reference") (OtherActor :type "Actor Object Reference") (OtherComp :type "PrimitiveComponent Object Reference") (OtherBodyIndex :type Integer) (bFromSweep :type Boolean) (SweepResult :type "HitResult Structure (by ref)"))
  (if (`KismetMathLibrary.ClassIsChildOf` (`GameplayStatics.GetObjectClass` OtherActor) "/Game/Blueprints/BP_Plane.BP_Plane_C")
    (set `self.Player` OtherActor)
    (`KismetSystemLibrary.K2_SetTimer` null "AAFire" 0.15 true)))

(event `self.PlayerNearby.OnComponentEndOverlap`
  (params (OverlappedComponent :type "PrimitiveComponent Object Reference") (OtherActor :type "Actor Object Reference") (OtherComp :type "PrimitiveComponent Object Reference") (OtherBodyIndex :type Integer))
  (if (`KismetMathLibrary.ClassIsChildOf` (`GameplayStatics.GetObjectClass` OtherActor) "/Game/Blueprints/BP_Plane.BP_Plane_C")
    (`KismetSystemLibrary.K2_ClearTimer` null "AAFire")))

(fn `AAFire`
  (bind _returnvalue (`SceneComponent.K2_GetComponentLocation` (`self.Arrow`)))
  (bind _outlaunchvelocity (`GameplayStatics.SuggestProjectileVelocity_MovingTarget` _returnvalue (`GameplayStatics.GetPlayerPawn` 0) (0.0 0.0 0.0) 0.0 0.25 "Persistent"))
  (`|SpawnActorFromClass` "/Game/Blueprints/BP_Enemy_Bullet.BP_Enemy_Bullet_C" (`KismetMathLibrary.MakeTransform` (+ _returnvalue (0.0 0.0 0.0)) (`KismetMathLibrary.MakeRotFromX` _outlaunchvelocity)) "Undefined" "MultiplyWithRoot" null (+ 0.0 20000.0) self)
  (`GameplayStatics.SpawnEmitterAtLocation` "/Game/StarterContent/Particles/P_Smoke.P_Smoke" (`SceneComponent.K2_GetComponentLocation` (`self.Arrow`)) (struct) (10.0 10.0 10.0)))

(fn `UserConstructionScript`
  (`parent.UserConstructionScript`))