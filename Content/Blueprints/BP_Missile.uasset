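; BP_Missile is a homing projectile that chases the target locked by the player's aircraft and explodes on impact.
; On BeginPlay it casts the player pawn to BP_Plane, or failing that BP_Attacker, and sets ProjectileMovement's homing target to a scene component of that pawn's LockedTarget, printing its name.
; On Hit it spawns an explosion emitter and applies fixed damage to the hit actor.
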(event `self.ReceiveBeginPlay`
  (bind _returnvalue (`GameplayStatics.GetPlayerPawn` 0))
  (bind _asbp_plane (cast `/Game/Blueprints/BP_Plane` _returnvalue)
    (:`then`
      (bind _output_get (set `ProjectileMovementComponent.HomingTargetComponent` (`self.GetComponentByClass` (`/Game/Blueprints/BP_Plane.LockedTarget` _asbp_plane) "/Script/Engine.SceneComponent") (`self.ProjectileMovement`))))
    (:`CastFailed`
      (bind _asbp_attacker (cast `/Game/Blueprints/BP_Attacker` _returnvalue))
      (set `ProjectileMovementComponent.HomingTargetComponent` (`self.GetComponentByClass` (`/Game/Blueprints/BP_Attacker.LockedTarget` _asbp_attacker) "/Script/Engine.SceneComponent") (`self.ProjectileMovement`))))
  (`KismetSystemLibrary.PrintString` (`KismetSystemLibrary.GetDisplayName` _output_get)))

(event `self.ReceiveHit`
  (params (MyComp :type "PrimitiveComponent Object Reference") (Other :type "Actor Object Reference") (OtherComp :type "PrimitiveComponent Object Reference") (bSelfMoved :type Boolean) (HitLocation :type "Vector Structure") (HitNormal :type "Vector Structure") (NormalImpulse :type "Vector Structure") (Hit :type "HitResult Structure (by ref)"))
  (`GameplayStatics.SpawnEmitterAtLocation` "/Game/StarterContent/Particles/P_Explosion.P_Explosion" HitLocation)
  (`GameplayStatics.ApplyDamage` Other 50.0))

(fn `UserConstructionScript`)