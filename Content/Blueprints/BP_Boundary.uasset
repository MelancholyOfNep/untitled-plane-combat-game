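; BP_Boundary marks the combat area and punishes planes that stay outside it.
; When a BP_Plane ends overlap, it prints a warning and starts a ten-second timer by function name.
; Re-entering clears that timer and prints a confirmation; otherwise OutOfBounds applies heavy damage.
; The damage always targets player pawn 0, whichever plane left the area.
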(event `self.ReceiveActorEndOverlap`
  (params (OtherActor :type "Actor Object Reference"))
  (if (`KismetMathLibrary.ClassIsChildOf` (`GameplayStatics.GetObjectClass` OtherActor) "/Game/Blueprints/BP_Plane.BP_Plane_C")
    (`KismetSystemLibrary.PrintString` "Out of bounds! You have 10 seconds to return to the combat area!")
    (bind _returnvalue (`KismetSystemLibrary.K2_SetTimer` null "OutOfBounds" 10.0))))

(event `self.ReceiveActorBeginOverlap`
  (params (OtherActor :type "Actor Object Reference"))
  (if (`KismetMathLibrary.ClassIsChildOf` (`GameplayStatics.GetObjectClass` OtherActor) "/Game/Blueprints/BP_Plane.BP_Plane_C")
    (`KismetSystemLibrary.K2_ClearAndInvalidateTimerHandle` (stale `self.ReceiveActorEndOverlap` _returnvalue))
    (`KismetSystemLibrary.PrintString` "You've returned to the combat area.")))

(fn `OutOfBounds`
  (`GameplayStatics.ApplyDamage` (`GameplayStatics.GetPlayerPawn` 0) 1000.0))

(fn `UserConstructionScript`)