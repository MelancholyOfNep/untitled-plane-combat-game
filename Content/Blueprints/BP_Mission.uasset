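; BP_Mission tracks priority objectives for a mission and returns to the MainMenu level once they are destroyed.
; BeginPlay casts to BP_GameInstance and zeroes its PriorityCount, printing debug messages along the way.
; PriorityDestroyed decrements the mission's own PriorityCount, separate from the GameInstance value, then opens MainMenu at zero or below, otherwise printing the remaining count.
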(event `self.ReceiveBeginPlay`
  (`KismetSystemLibrary.PrintString` "Hello")
  (bind _asbp_game_instance (cast `/Game/Blueprints/BP_GameInstance` (`GameplayStatics.GetGameInstance`))
    (:`then`
      (`KismetSystemLibrary.PrintString` "Before")
      (set `/Game/Blueprints/BP_GameInstance.PriorityCount` 0 _asbp_game_instance)
      (`KismetSystemLibrary.PrintString` "After"))
    (:`CastFailed`
      (`KismetSystemLibrary.PrintString` "Fail"))))

(event `PriorityDestroyed`
  (bind _result (`/Engine/EditorBlueprintResources/StandardMacros.DecrementInt` (stale _output_get))
    (:`  `
      (bind _output_get (set `self.PriorityCount` _result))
      (if (<= _output_get 0)
        (`GameplayStatics.OpenLevel` "MainMenu")
        (else
          (`KismetSystemLibrary.PrintString` (`KismetStringLibrary.Conv_IntToString` _output_get)))))))

(fn `UserConstructionScript`)