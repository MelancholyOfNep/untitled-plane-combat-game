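; BP_Bullet is a projectile actor that damages characters it hits and explodes on impact.
; The construction script copies its Speed variable into the ProjectileMovement initial and max speed.
; On Hit, it applies fixed damage if the other actor is a child of the test enemy, friendly or patrol enemy classes.
; Any hit then spawns an explosion emitter and sound at the impact point and destroys the bullet.
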(event `self.ReceiveHit`
  (params (MyComp :type "PrimitiveComponent Object Reference") (Other :type "Actor Object Reference") (OtherComp :type "PrimitiveComponent Object Reference") (bSelfMoved :type Boolean) (HitLocation :type "Vector Structure") (HitNormal :type "Vector Structure") (NormalImpulse :type "Vector Structure") (Hit :type "HitResult Structure (by ref)"))
  (bind _returnvalue (`GameplayStatics.GetObjectClass` Other))
  (if (`KismetMathLibrary.ClassIsChildOf` _returnvalue "/Game/Blueprints/BP_EnemyTest.BP_EnemyTest_C")
    (`GameplayStatics.ApplyDamage` Other 10.0 :!label _label)
    (elif (`KismetMathLibrary.ClassIsChildOf` _returnvalue "/Game/Blueprints/BP_Friendly.BP_Friendly_C")
      (goto _label)
      (elif (`KismetMathLibrary.ClassIsChildOf` _returnvalue "/Game/Blueprints/BP_Patrol_enemy.BP_Patrol_enemy_C")
        (goto _label)
        (else
          _))))
  (`GameplayStatics.SpawnEmitterAtLocation` "/Game/StarterContent/Particles/P_Explosion.P_Explosion" HitLocation)
  (`GameplayStatics.PlaySoundAtLocation` "/Game/StarterContent/Audio/Explosion02.Explosion02" HitLocation (struct) 0.1 1.0 0.0 null null null null)
  (`self.K2_DestroyActor`))

(fn `UserConstructionScript`
  (bind _projectilemovement (`self.ProjectileMovement`))
  (bind _output_get (set `ProjectileMovementComponent.InitialSpeed` (`self.Speed`) _projectilemovement))
  (set `ProjectileMovementComponent.MaxSpeed` _output_get _projectilemovement))