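; BP_Bomb is a bomb actor that explodes on impact, dealing radial damage over a wide area.
; Each Tick it blends its rotation toward its velocity, so it faces the direction of travel.
; On Hit it applies falloff damage from just above the impact point, sparing the player pawn and letting static world geometry block it.
; It then spawns a heavily scaled explosion emitter and destroys itself.
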(event `self.ReceiveTick`
  (params (DeltaSeconds :type "Float (single-precision)"))
  (bind _returnvalue (`self.K2_GetActorLocation`))
  (`self.K2_SetActorRotation` (`KismetMathLibrary.RLerp` (`self.K2_GetActorRotation`) (`KismetMathLibrary.FindLookAtRotation` _returnvalue (+ _returnvalue (`self.GetVelocity`))) 0.9)))

(event `self.ReceiveHit`
  (params (MyComp :type "PrimitiveComponent Object Reference") (Other :type "Actor Object Reference") (OtherComp :type "PrimitiveComponent Object Reference") (bSelfMoved :type Boolean) (HitLocation :type "Vector Structure") (HitNormal :type "Vector Structure") (NormalImpulse :type "Vector Structure") (Hit :type "HitResult Structure (by ref)"))
  (`GameplayStatics.ApplyRadialDamageWithFalloff` 100.0 10.0 (+ Hit_Location (0.0 0.0 10.0)) 100.0 5000.0 1.0 null (`|MakeArray` (`GameplayStatics.GetPlayerPawn` 0) :!type "Actor Object Reference") self null "ECC_WorldStatic")
  (`GameplayStatics.SpawnEmitterAtLocation` "/Game/StarterContent/Particles/P_Explosion.P_Explosion" Hit_Location (struct) (500.0 500.0 500.0))
  (`self.K2_DestroyActor`))

(fn `UserConstructionScript`)