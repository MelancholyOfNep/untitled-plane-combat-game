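; BP_EnemyTest is a destructible enemy target with a HUD marker, colored red for priority targets and green for normal ones.
; On BeginPlay, priority targets add to the GameInstance's priority count and show their target text.
; Damage depletes Health; death reports to the GameInstance, plays explosion effects, awards money and clears the player plane's lock.
; Locked and Unlocked events toggle the marker's current-target indicator.
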(event `self.ReceiveBeginPlay`
  (bind _hudmarker (`self.HUDmarker`))
  (bind _returnvalue (`WidgetComponent.GetUserWidgetObject` _hudmarker))
  (`KismetSystemLibrary.Delay` 0.2)
  (if (`self.IsPriority`)
    (bind _asbp_game_instance (cast `/Game/Blueprints/BP_GameInstance` (`GameplayStatics.GetGameInstance`)))
    (bind _result (`/Engine/EditorBlueprintResources/StandardMacros.IncrementInt` (stale _output_get))
      (:`  `
        (bind _output_get (set `/Game/Blueprints/BP_GameInstance.PriorityCount` _result _asbp_game_instance))
        (`KismetSystemLibrary.PrintString` (`KismetStringLibrary.Conv_IntToString` _output_get))
        (`UserWidget.SetColorAndOpacity` _returnvalue (struct :`R` 1.0 :`A` 0.75))
        (bind _aswbp_enemy_highlight (cast `/Game/Blueprints/HUD/WBP_EnemyHighlight` (`WidgetComponent.GetWidget` _hudmarker)))
        (`TextBlock.SetOpacity` (`/Game/Blueprints/HUD/WBP_EnemyHighlight.TGT_Text` _aswbp_enemy_highlight) 1.0)))
    (else
      (`UserWidget.SetColorAndOpacity` _returnvalue (struct :`G` 1.0 :`B` 0.113694 :`A` 1.0)))))

(event `self.ReceiveAnyDamage`
  (params (Damage :type "Float (single-precision)") (DamageType :type "DamageType Object Reference") (InstigatedBy :type "Controller Object Reference") (DamageCauser :type "Actor Object Reference"))
  (bind _returnvalue (`GameplayStatics.GetGameInstance`))
  (bind _enemytype (`self.EnemyType`))
  (bind _value (`self.Value`))
  (bind _returnvalue_2 (`SceneComponent.K2_GetComponentLocation` (`self.Box`)))
  (bind _output_get (set `self.Health` (- (stale _output_get) Damage)))
  (if (<= _output_get 0.0)
    (if (`self.IsPriority`)
      (bind _asbp_game_instance (cast `/Game/Blueprints/BP_GameInstance` _returnvalue))
      (`/Game/Blueprints/BP_GameInstance.PriorityDestroyed` _asbp_game_instance _enemytype _value)
      (else
        (bind _asbp_game_instance_2 (cast `/Game/Blueprints/BP_GameInstance` _returnvalue))
        (`/Game/Blueprints/BP_GameInstance.NormalDestroyed` _asbp_game_instance_2 _enemytype _value)))
    (`GameplayStatics.PlaySoundAtLocation` "/Game/StarterContent/Audio/Explosion01.Explosion01" _returnvalue_2 (struct) 1.0 1.0 0.0 null null null null)
    (`NiagaraFunctionLibrary.SpawnSystemAtLocation` "/Game/M5VFXVOL2/Niagara/Explosion/NFire_Exp_03.NFire_Exp_03" _returnvalue_2 (struct) (2.0 2.0 2.0))
    (`self.K2_DestroyActor`)
    (bind _asbp_game_instance_3 (cast `/Game/Blueprints/BP_GameInstance` (`GameplayStatics.GetGameInstance`)))
    (bind _output_get_2 (set `/Game/Blueprints/BP_GameInstance.Money` (+ (stale _output_get_2) (`self.Value`)) _asbp_game_instance_3))
    (`KismetSystemLibrary.PrintString` (`KismetStringLibrary.Concat_StrStr` "Target Destroyed! Money: " (`KismetStringLibrary.Conv_IntToString` _output_get_2)))
    (bind _asbp_plane (cast `/Game/Blueprints/BP_Plane` (`GameplayStatics.GetPlayerPawn` 0)))
    (if (== (`/Game/Blueprints/BP_Plane.LockedTarget` _asbp_plane) self)
      (set `/Game/Blueprints/BP_Plane.LockedTarget` null _asbp_plane))))

(event `Locked`
  (bind _aswbp_enemy_highlight (cast `/Game/Blueprints/HUD/WBP_EnemyHighlight` (`WidgetComponent.GetWidget` (`self.HUDmarker`))))
  (`Image.SetOpacity` (`/Game/Blueprints/HUD/WBP_EnemyHighlight.CurrentTarget` _aswbp_enemy_highlight) 1.0))

(event `Unlocked`
  (bind _aswbp_enemy_highlight (cast `/Game/Blueprints/HUD/WBP_EnemyHighlight` (`WidgetComponent.GetWidget` (`self.HUDmarker`))))
  (`Image.SetOpacity` (`/Game/Blueprints/HUD/WBP_EnemyHighlight.CurrentTarget` _aswbp_enemy_highlight) 0.0))

(fn `UserConstructionScript`)