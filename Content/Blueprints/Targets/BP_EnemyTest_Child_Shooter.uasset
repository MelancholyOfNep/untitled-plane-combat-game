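; An anti-aircraft turret enemy, a child Blueprint that tracks and shoots at a plane inside its PlayerNearby trigger.
; Overlaps set the tracking flag, and a BP_Plane also starts or clears a looping fire timer.
; Tick lerps the turret skeleton's yaw toward the stored plane.
; AAFire spawns bullets from the arrow along a predicted moving-target velocity toward player pawn 0, with gunshot sound and explosion effect.
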(event `self.ReceiveTick`
  (params (DeltaSeconds :type "Float (single-precision)"))
  (bind _turretskele (`self.turretskele`))
  (bind (_returnvalue_roll _returnvalue_pitch _returnvalue_yaw) (`KismetMathLibrary.BreakRotator` (`SceneComponent.K2_GetComponentRotation` _turretskele)))
  (`parent.ReceiveTick` DeltaSeconds)
  (if (stale `self.PlayerNearby.OnComponentBeginOverlap` _output_get)
    (bind (_returnvalue_roll_2 _returnvalue_pitch_2 _returnvalue_yaw_2) (`KismetMathLibrary.BreakRotator` (`KismetMathLibrary.FindLookAtRotation` (`SceneComponent.K2_GetComponentLocation` _turretskele) (`self.K2_GetActorLocation` (stale `self.PlayerNearby.OnComponentBeginOverlap` _output_get_2)))))
    (`SceneComponent.K2_SetWorldRotation` (`self.turretskele`) (`KismetMathLibrary.MakeRotator` _returnvalue_roll _returnvalue_pitch (`KismetMathLibrary.Lerp` _returnvalue_yaw _returnvalue_yaw_2 0.2)) false false)))

(event `self.PlayerNearby.OnComponentBeginOverlap`
  (params (OverlappedComponent :type "PrimitiveComponent Object Reference") (OtherActor :type "Actor Object Reference") (OtherComp :type "PrimitiveComponent Object Reference") (OtherBodyIndex :type Integer) (bFromSweep :type Boolean) (SweepResult :type "HitResult Structure (by ref)"))
  (bind _output_get (set `self.PlayerNear?` true))
  (if (`KismetMathLibrary.ClassIsChildOf` (`GameplayStatics.GetObjectClass` OtherActor) "/Game/Blueprints/BP_Plane.BP_Plane_C")
    (bind _output_get_2 (set `self.Player` OtherActor))
    (`KismetSystemLibrary.K2_SetTimer` null "AAFire" 0.15 true)))

(event `self.PlayerNearby.OnComponentEndOverlap`
  (params (OverlappedComponent :type "PrimitiveComponent Object Reference") (OtherActor :type "Actor Object Reference") (OtherComp :type "PrimitiveComponent Object Reference") (OtherBodyIndex :type Integer))
  (set `self.PlayerNear?` false)
  (if (`KismetMathLibrary.ClassIsChildOf` (`GameplayStatics.GetObjectClass` OtherActor) "/Game/Blueprints/BP_Plane.BP_Plane_C")
    (`KismetSystemLibrary.K2_ClearTimer` null "AAFire")))

(fn `AAFire`
  (bind _returnvalue (`SceneComponent.K2_GetComponentLocation` (`self.Arrow`)))
  (bind _returnvalue_2 (`SceneComponent.K2_GetComponentLocation` (`self.Arrow`)))
  (bind _outlaunchvelocity (`GameplayStatics.SuggestProjectileVelocity_MovingTarget` _returnvalue_2 (`GameplayStatics.GetPlayerPawn` 0) (0.0 0.0 0.0) 0.0 0.25 "None"))
  (`|SpawnActorFromClass` "/Game/Blueprints/BP_Enemy_Bullet.BP_Enemy_Bullet_C" (`KismetMathLibrary.MakeTransform` (+ _returnvalue_2 (0.0 0.0 0.0)) (`KismetMathLibrary.MakeRotFromX` _outlaunchvelocity)) "Undefined" "MultiplyWithRoot" null (+ 0.0 20000.0) self)
  (`GameplayStatics.PlaySoundAtLocation` "/Game/Audio/SFX/536630__snapssound__gunshot_01sse.536630__snapssound__gunshot_01sse" _returnvalue (struct) 0.15 1.0 0.0 null null null null)
  (`GameplayStatics.SpawnEmitterAtLocation` "/Game/StarterContent/Particles/P_Explosion.P_Explosion" _returnvalue (struct) (2.0 2.0 2.0)))

(fn `UserConstructionScript`
  (`parent.UserConstructionScript`))